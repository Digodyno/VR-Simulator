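; Test ship Blueprint driven by keyboard, with a seven-position engine telegraph on W/S and speed, compass and M-key flow/wind widgets.
; Tick eases ForwardVelocity toward the gear's target and updates the speed display; axis inputs apply it as force and speed-scaled torque.
; A looping timer saves serial knob and wheel values, restored on BeginPlay but not used for movement.
; SerialPortHandler is never called here, and the compass arrow update is disconnected.
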(event `Key|M`
  (params (Key :type "Key Structure"))
  (:`Released`
    (if (not (`Widget.IsInViewport` (stale `self.ReceiveBeginPlay` _returnvalue)))
      (`UserWidget.AddToViewport` (stale `self.ReceiveBeginPlay` _returnvalue) 0))))

(event `self.ReceiveBeginPlay`
  (`self.LoadGame`)
  (`KismetSystemLibrary.K2_SetTimer` null "SaveGame" 5.0 true)
  (`|ExecutionSequence`
    (:`then_0`
      (bind _returnvalue (`|CreateWidget` "/Game/UI/UI_Flow+Wind.UI_Flow+Wind_C" (`GameplayStatics.GetPlayerController` 0))))
    (:`then_1`
      (bind _returnvalue_2 (`|CreateWidget` "/Game/UI/UI_compass.UI_compass_C"))
      (bind _output_get (set `self.Compass REF` _returnvalue_2))
      (`UserWidget.AddToViewport` _output_get 0)
      (bind _outactors (`GameplayStatics.GetAllActorsOfClass` "/Game/UI/north_marker.north_marker_C"))
      (bind _returnvalue_3 (`GameplayStatics.GetActorArrayAverageLocation` _outactors))
      (set `self.North Location` _returnvalue_3))
    (:`then_2`
      (bind _returnvalue_4 (`|CreateWidget` "/Game/UI/UI_Speed.UI_Speed_C"))
      (bind _output_get_2 (set `self.SpeedUI` _returnvalue_4))
      (`UserWidget.AddToViewport` _output_get_2 0))))

(event `InputAxis|Right_Left`
  (params (AxisValue :type "Float (single-precision)"))
  (bind _forwardvelocity_x (`KismetMathLibrary.BreakVector` (`self.ForwardVelocity`)))
  (bind _returnvalue (* AxisValue _forwardvelocity_x))
  ;[1 1 1] Keyboard movement (on for now)
  (`PrimitiveComponent.AddTorqueInRadians` (`self.mesh`) (`KismetMathLibrary.MakeVector` (* _returnvalue 10.0) 0.0 (* _returnvalue 5.0)) "None" false))

(event `InputAxis|Forward_Back`
  (params (AxisValue :type "Float (single-precision)"))
  ;[1 1 1] Keyboard movement (on for now)
  (`PrimitiveComponent.AddForce` (`self.mesh`) (* (`self.GetActorForwardVector`) (`self.ForwardVelocity`)) "None" false))

(event `self.ReceiveTick`
  (params (DeltaSeconds :type "Float (single-precision)"))
  (bind _forwardvelocity_x (`KismetMathLibrary.BreakVector` (`self.ForwardVelocity`)))
  (bind _forwardvelocity_x_2 (`KismetMathLibrary.BreakVector` (`self.ForwardVelocity`)))
  (bind _knobmultiplyer (`self.knobMultiplyer`))
  (bind _returnvalue (* (`self.defaultSpeed`) _knobmultiplyer))
  (bind _returnvalue_2 (* _forwardvelocity_x_2 (+ (`KismetMathLibrary.Abs` _knobmultiplyer) 1.0) 5e-06))
  (bind _returnvalue_3 (- _forwardvelocity_x_2 _returnvalue_2))
  (bind _returnvalue_4 (* (+ (`KismetMathLibrary.Abs` _returnvalue) (`KismetMathLibrary.Abs` _forwardvelocity_x_2)) 0.0009))
  (bind _returnvalue_5 (- _forwardvelocity_x_2 _returnvalue_4))
  (bind _returnvalue_6 (+ _returnvalue_4 _forwardvelocity_x_2))
  (bind _returnvalue_7 (+ _returnvalue_3 (* _returnvalue_2 0.05)))
  ;[1 1 1] Keyboard movement (on for now)
  (`/Engine/EditorBlueprintResources/StandardMacros.CompareFloat` _knobmultiplyer 1e-06
    (:`>`
      (if (<= _forwardvelocity_x_2 _returnvalue)
        (set `self.ForwardVelocity` (`KismetMathLibrary.MakeVector` _returnvalue_6 _returnvalue_6))
        (else
          (set `self.ForwardVelocity` (`KismetMathLibrary.MakeVector` _returnvalue_7 _returnvalue_7) :!label _label))))
    (:`==`
      (set `self.ForwardVelocity` (`KismetMathLibrary.MakeVector` _returnvalue_3 _returnvalue_3)))
    (:`<`
      (if (<= _returnvalue _forwardvelocity_x_2)
        (set `self.ForwardVelocity` (`KismetMathLibrary.MakeVector` _returnvalue_5 _returnvalue_5))
        (else
          (goto _label)))))
  (`TextBlock.SetText` (`/Game/UI/UI_Speed.TextSpeed` (`self.SpeedUI`)) (`KismetTextLibrary.Conv_DoubleToText` (/ _forwardvelocity_x (`self.defaultSpeed`)) "HalfToEven" false true 1 324 1 1))
  (`KismetSystemLibrary.PrintString` (`KismetStringLibrary.Conv_DoubleToString` _returnvalue_3)))

(event `Key|W`
  (params (Key :type "Key Structure"))
  (bind _knobposition (`self.knobPosition`))
  ;[1 1 1] Keyboard movement (on for now)
  (:`Pressed`
    (`/Engine/EditorBlueprintResources/StandardMacros.CompareInt` _knobposition 6
      (:`<`
        (bind _result (`/Engine/EditorBlueprintResources/StandardMacros.IncrementInt` _knobposition)
          (:`  `
            (set `self.knobPosition` _result)
            (switch `int` _knobposition :!label _label_2
              (:`Default`
                (set `self.knobMultiplyer` 0.0 :!label _label_3)
                (set `self.GearText` "Нейтраль"))
              (:`0`
                (set `self.knobMultiplyer` -6.0)
                (set `self.GearText` "Полный назад"))
              (:`1`
                (set `self.knobMultiplyer` -5.0)
                (set `self.GearText` "Крейсерская скорость (назад)"))
              (:`2`
                (set `self.knobMultiplyer` -1.5)
                (set `self.GearText` "Малый назад"))
              (:`3`
                (goto _label_3))
              (:`4`
                (set `self.knobMultiplyer` 2.0)
                (set `self.GearText` "Малый вперед"))
              (:`5`
                (set `self.knobMultiplyer` 6.0)
                (set `self.GearText` "Крейсерская скорость (вперед)"))
              (:`6`
                (set `self.knobMultiplyer` 7.0)
                (set `self.GearText` "Полный вперед")))
            (`TextBlock.SetText` (`/Game/UI/UI_Speed.TextKnots` (`self.SpeedUI`)) (`KismetTextLibrary.Conv_StringToText` (`self.GearText`)))))))))

(event `Key|S`
  (params (Key :type "Key Structure"))
  (bind _knobposition (`self.knobPosition`))
  ;[1 1 1] Keyboard movement (on for now)
  (:`Pressed`
    (`/Engine/EditorBlueprintResources/StandardMacros.CompareInt` _knobposition
      (:`>`
        (bind _result (`/Engine/EditorBlueprintResources/StandardMacros.DecrementInt` _knobposition)
          (:`  `
            (set `self.knobPosition` _result)
            (goto _label_2)))))))

(fn `LoadGame`
  (bind _saveslotname (`self.saveSlotName`))
  (bind _returnvalue (`GameplayStatics.DoesSaveGameExist` _saveslotname))
  (if _returnvalue
    (bind _returnvalue_2 (`GameplayStatics.LoadGameFromSlot` _saveslotname))
    (bind _assave_parameters_bp (cast `/Game/Ship/SaveParameters_BP` _returnvalue_2))
    (set `self.CurrentWheelValue` (`/Game/Ship/SaveParameters_BP.CurrentWheelValueSave` _assave_parameters_bp))
    (set `self.CurrentKnobValue` (`/Game/Ship/SaveParameters_BP.CurrentKnobValueSave` _assave_parameters_bp))))

(fn `SaveGame`
  (bind _returnvalue (`GameplayStatics.CreateSaveGameObject` "/Game/Ship/SaveParameters_BP.SaveParameters_BP_C"))
  (bind _output_get (set `self.GameSaver` _returnvalue))
  (set `/Game/Ship/SaveParameters_BP.CurrentWheelValueSave` (`self.CurrentWheelValue`) _output_get)
  (set `/Game/Ship/SaveParameters_BP.CurrentKnobValueSave` (`self.CurrentKnobValue`) _output_get)
  (`GameplayStatics.SaveGameToSlot` (`self.GameSaver`) (`self.saveSlotName`)))

(fn `SerialPortHandler`
  (bind _returnvalue (`KismetStringLibrary.Conv_StringToInt` (`self.SerialKnobRead`)))
  (set `self.PrevKnobValue` (`self.CurrentKnobValue`))
  (set `self.PrevWheelValue` (`self.CurrentWheelValue`))
  (set `self.SerialPortInput` _returnvalue)
  (set `self.CurrentKnobValue` _returnvalue)
  (set `self.CurrentWheelValue` (`KismetStringLibrary.Conv_StringToInt` (`self.SerislWheelRead`))))

(fn `UserConstructionScript`)