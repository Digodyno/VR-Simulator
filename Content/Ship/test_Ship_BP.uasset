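; Test ship Blueprint that the player steers, with speed and yaw offset by flow and wind values.
; Keyboard axes accumulate velocity and yaw to drive a center-of-mass force and controller yaw; parallel functions do the same from serial knob and wheel deltas, uncalled here.
; BeginPlay loads saved knob/wheel values, starts timed autosaving and creates a compass pointing at averaged North_marker locations, plus a FlowWind widget shown with M.
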(event `self.ReceiveTick`
  (params (DeltaSeconds :type "Float (single-precision)"))
  (bind (_returnvalue_roll _returnvalue_pitch _returnvalue_yaw) (`KismetMathLibrary.BreakRotator` (`self.GetControlRotation`)))
  (bind (_returnvalue_roll_2 _returnvalue_pitch_2 _returnvalue_yaw_2) (`KismetMathLibrary.BreakRotator` (`KismetMathLibrary.FindLookAtRotation` (`self.K2_GetActorLocation`) (`self.North Location`))))
  (`Widget.SetRenderTransformAngle` (`/Game/UI/UI_compass.compass_arrow` (`self.Compass REF`)) (- _returnvalue_yaw _returnvalue_yaw_2)))

(event `Key|M`
  (params (Key :type "Key Structure"))
  (:`Released`
    (if (not (`Widget.IsInViewport` (stale `self.ReceiveBeginPlay` _returnvalue)))
      (`UserWidget.AddToViewport` (stale `self.ReceiveBeginPlay` _returnvalue) 0))))

(event `self.ReceiveBeginPlay`
  (`self.LoadGame`)
  (`KismetSystemLibrary.K2_SetTimer` null "SaveGame" 5.0 true)
  (`|ExecutionSequence`
    (:`then_0`
      (bind _returnvalue (`|CreateWidget` "/Game/UI/UI_Flow+Wind.UI_Flow+Wind_C" (`GameplayStatics.GetPlayerController` 0))))
    (:`then_1`
      (bind _returnvalue_2 (`|CreateWidget` "/Game/UI/UI_compass.UI_compass_C"))
      (bind _output_get (set `self.Compass REF` _returnvalue_2))
      (`UserWidget.AddToViewport` _output_get 0)
      (bind _outactors (`GameplayStatics.GetAllActorsOfClass` "/Game/UI/north_marker.north_marker_C"))
      (bind _returnvalue_3 (`GameplayStatics.GetActorArrayAverageLocation` _outactors))
      (set `self.North Location` _returnvalue_3))))

(event `Key|A`
  (params (Key :type "Key Structure"))
  ;[1 1 1] Keyboard movement (on for now)
  (:`Released`
    (bind _output_get (set `self.Yaw` (+ (* (+ (stale `InputAxis|Right_Left` AxisValue) (`self.XFlow`) (`self.XWind`)) 0.0005) (`self.Yaw`)) :!label _label))
    (`self.AddControllerYawInput` _output_get)))

(event `Key|D`
  (params (Key :type "Key Structure"))
  ;[1 1 1] Keyboard movement (on for now)
  (:`Released`
    (goto _label)))

(event `Key|SpaceBar`
  (params (Key :type "Key Structure"))
  ;[1 1 1] Keyboard movement (on for now)
  (:`Released`
    (set `self.Velocity` 0.0)))

(event `InputAxis|Right_Left`
  (params (AxisValue :type "Float (single-precision)"))
  ;[1 1 1] Keyboard movement (on for now)
  (goto _label))

(event `InputAxis|Forward_Back`
  (params (AxisValue :type "Float (single-precision)"))
  (bind (_returnvalue_x _returnvalue_y) (`KismetMathLibrary.BreakVector` (`self.GetActorForwardVector`)))
  ;[1 1 1] Keyboard movement (on for now)
  (bind _output_get (set `self.Velocity` (+ (* AxisValue (`self.Acceleration`)) (`self.Velocity`))))
  (bind _output_get_2 (set `self.YSpeed` (+ _output_get (`self.YFlow`) (`self.YWind`))))
  (`PrimitiveComponent.AddForceAtLocation` (`self.CollisionComponent`) (* (* (`KismetMathLibrary.MakeVector` _returnvalue_x _returnvalue_y) _output_get_2) 0.001) (`PrimitiveComponent.GetCenterOfMass` (`self.CollisionComponent`) "None") "None"))

(fn `LoadGame`
  (bind _saveslotname (`self.saveSlotName`))
  (bind _returnvalue (`GameplayStatics.DoesSaveGameExist` _saveslotname))
  (if _returnvalue
    (bind _returnvalue_2 (`GameplayStatics.LoadGameFromSlot` _saveslotname))
    (bind _assave_parameters_bp (cast `/Game/Ship/SaveParameters_BP` _returnvalue_2))
    (set `self.CurrentWheelValue` (`/Game/Ship/SaveParameters_BP.CurrentWheelValueSave` _assave_parameters_bp))
    (set `self.CurrentKnobValue` (`/Game/Ship/SaveParameters_BP.CurrentKnobValueSave` _assave_parameters_bp))))

(fn `SaveGame`
  (bind _returnvalue (`GameplayStatics.CreateSaveGameObject` "/Game/Ship/SaveParameters_BP.SaveParameters_BP_C"))
  (bind _output_get (set `self.GameSaver` _returnvalue))
  (set `/Game/Ship/SaveParameters_BP.CurrentWheelValueSave` (`self.CurrentWheelValue`) _output_get)
  (set `/Game/Ship/SaveParameters_BP.CurrentKnobValueSave` (`self.CurrentKnobValue`) _output_get)
  (`GameplayStatics.SaveGameToSlot` (`self.GameSaver`) (`self.saveSlotName`)))

(fn `SerialPortHandler`
  (bind _returnvalue (`KismetStringLibrary.Conv_StringToInt` (`self.SerialKnobRead`)))
  (set `self.PrevKnobValue` (`self.CurrentKnobValue`))
  (set `self.PrevWheelValue` (`self.CurrentWheelValue`))
  (set `self.SerialPortInput` _returnvalue)
  (set `self.CurrentKnobValue` _returnvalue)
  (set `self.CurrentWheelValue` (`KismetStringLibrary.Conv_StringToInt` (`self.SerislWheelRead`))))

(fn `SetKnob`
  (bind (_returnvalue_x _returnvalue_y) (`KismetMathLibrary.BreakVector` (`self.GetActorForwardVector`)))
  (bind _output_get (set `self.Velocity` (+ (* (- (`KismetMathLibrary.Conv_IntToDouble` (`self.PrevKnobValue`)) (`KismetMathLibrary.Conv_IntToDouble` (`self.CurrentKnobValue`))) (`self.Acceleration`)) (`self.Velocity`))))
  (bind _output_get_2 (set `self.YSpeed` (+ _output_get (`self.YFlow`) (`self.YWind`))))
  (`PrimitiveComponent.AddForceAtLocation` (`self.CollisionComponent`) (* (`KismetMathLibrary.MakeVector` _returnvalue_x _returnvalue_y) _output_get_2) (`PrimitiveComponent.GetCenterOfMass` (`self.CollisionComponent`) "None") "None"))

(fn `SetSteeringWheel`
  (bind _output_get (set `self.Yaw` (+ (* (- (`KismetMathLibrary.Conv_IntToDouble` (`self.PrevWheelValue`)) (`KismetMathLibrary.Conv_IntToDouble` (`self.CurrentWheelValue`))) 0.0005) (`self.Yaw`) (`self.XFlow`) (`self.XWind`))))
  (`self.AddControllerYawInput` _output_get))

(fn `show_ui_vidjet`
  (params (Class :type "UserWidget Class Reference"))
  (`WidgetLayoutLibrary.RemoveAllWidgets`)
  (bind _returnvalue (`|CreateWidget` Class (`GameplayStatics.GetPlayerController` 0)))
  (`UserWidget.AddToViewport` _returnvalue 0))

(fn `UserConstructionScript`)